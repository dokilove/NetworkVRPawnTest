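; Lobby GameMode that keeps track of players as they log in.
; On each PostLogin it sets UserCount on BP_LobbyGS from the length of its PlayerArray.
; With authority, it calls OnRepUserCount directly on the game state and adds the new player to AllPlayerControllers.
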(event EventBeginPlay)

(event EventTick
  (params (DeltaSeconds :type Float%20%28single-precision%29)))

(event EventPostLogin
  (params (NewPlayer :type Player%20Controller%20Object%20Reference))
  ;[1 1 1] 플레이어가 한명씩 로그인할 때마다 BP_LobbyGS의 UserCount를 늘리는 함수를 호출 이거 나중에 배웁니다 신경쓰지 마세요
  (bind _asbp_lobby_gs (Utilities|Casting|CastToBP_LobbyGS (Game|GetGameState)))
  (Utilities|IsValid _asbp_lobby_gs
    (:Is%20Valid
      (Variables|/Game/Blueprints/Lobby/BP_LobbyGS.BP_LobbyGS_C|SetUserCount _asbp_lobby_gs (Utilities|Array|Length (Variables|/Script/Engine.GameStateBase|GetPlayerArray _asbp_lobby_gs)))
      (if (Ability|HasAuthority)
        (Default|OnRepUserCount _asbp_lobby_gs)
        (Utilities|Array|Add (Variables|Default|GetAllPlayerControllers) NewPlayer)))))

(fn ConstructionScript)