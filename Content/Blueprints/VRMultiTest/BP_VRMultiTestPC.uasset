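; BP_VRMultiTestPC is a test Blueprint, apparently a player controller, for switching VR on and off at runtime.
; It shows the mouse cursor on BeginPlay and offers EnableVR and DisableVR events that set HMD and stereo through console commands, in reverse order when disabling.
; Debug chains printing "E" and "Q" call these events but never run, so nothing in this Blueprint triggers the toggle.
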(event Custom|EnableVR
  (Development|ExecuteConsoleCommand "vr.bEnableHMD True" 0)
  (Development|ExecuteConsoleCommand "vr.bEnableStereo True" 0))

(event Custom|DisableVR
  (Development|ExecuteConsoleCommand "vr.bEnableStereo False" 0)
  (Development|ExecuteConsoleCommand "vr.bEnableHMD False" 0))

(event EventBeginPlay
  (Variables|Default|SetbShowMouseCursor true))

(event EventTick
  (params (DeltaSeconds :type Float%20%28single-precision%29)))

(event Input|KeyboardEvents|E
  (params (Key :type Key%20Structure)))

(event Input|KeyboardEvents|Q
  (params (Key :type Key%20Structure)))

(fn ConstructionScript)