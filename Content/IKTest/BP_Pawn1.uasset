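; VR pawn in an IK test folder that carries a skeletal mesh with the headset camera and records both hand transforms.
; BeginPlay sets the tracking origin per HMD, adding a height offset for PSVR, and spawns two motion controllers attached to the VR origin.
; Tick stores controller world transforms in hand variables and snaps the mesh to the camera's location and rotation.
; Grab inputs forward grab and release to the matching controller.
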(event EventTick
  (params (DeltaSeconds :type Float%20%28single-precision%29))
  (bind _rightcontroller (Variables|Default|GetRightController))
  (bind _camera (Variables|Default|GetCamera))
  (bind _leftcontroller (Variables|Default|GetLeftController))
  (Utilities|IsValid _rightcontroller
    (:Is%20Valid
      (Variables|Default|SetHandRTransform (Transformation|GetWorldTransform (Variables|/Game/IKTest/BP_MotionController.BP_MotionController_C|GetMotionController _rightcontroller)))
      (Utilities|IsValid _leftcontroller
        (:Is%20Valid
          (Variables|Default|SetHandLTransfrorm (Transformation|GetWorldTransform (Variables|/Game/IKTest/BP_MotionController.BP_MotionController_C|GetMotionController _leftcontroller)))
          (Transformation|SetWorldLocationAndRotation (Variables|Default|GetSkeletalMesh) (Transformation|GetWorldLocation _camera) (Transformation|GetWorldRotation _camera) false false))))))

(event EventBeginPlay
  (bind _returnvalue (Transformation|GetActorTransform))
  (bind _returnvalue_2 (Math|Transform|MakeTransform "0, 0, 0"))
  (bind _self self)
  (Utilities|FlowControl|Sequence
    (:then_0
      ;[1 1 1] Setup Player Height for various Platforms
      (switch name (Class|HeadMountedDisplayFunctionLibrary|GetHMDDeviceName)
        (:OculusHMD
          (Class|HeadMountedDisplayFunctionLibrary|SetTrackingOrigin "Floor" :!label _label))
        (:SteamVR
          (goto _label))
        (:PSVR
          (Class|HeadMountedDisplayFunctionLibrary|SetTrackingOrigin "Eye")
          (Transformation|AddLocalOffset (Variables|Default|GetVROrigin) (Math|Vector|MakeVector 0.0 0.0 (Variables|Default|GetDefaultPlayerHeight)) false false))))
    (:then_1
      ;[1 1 1] Spwan and attach both motion controllers
      (Utilities|FlowControl|Sequence
        (:then_0
          (bind _returnvalue_3 (Game|SpawnActorfromClass "/Game/IKTest/BP_MotionController.BP_MotionController_C" _returnvalue_2 "Undefined" _self "Left" 0))
          (bind _output_get (Variables|Default|SetLeftController _returnvalue_3))
          (Transformation|AttachComponentToComponent _returnvalue_3 (Variables|Default|GetVROrigin) "None" "SnapToTarget" "SnapToTarget" "KeepWorld" false)
          (Variables|Default|SetHandLTransfrorm (Transformation|GetWorldTransform (Variables|/Game/IKTest/BP_MotionController.BP_MotionController_C|GetMotionController _output_get))))
        (:then_1
          (bind _returnvalue_4 (Game|SpawnActorfromClass "/Game/IKTest/BP_MotionController.BP_MotionController_C" _returnvalue_2 "Undefined" _self "Right" 0))
          (bind _output_get_2 (Variables|Default|SetRightController _returnvalue_4))
          (Transformation|AttachComponentToComponent _returnvalue_4 (Variables|Default|GetVROrigin) "None" "SnapToTarget" "SnapToTarget" "KeepWorld" false)
          (Variables|Default|SetHandRTransform (Transformation|GetWorldTransform (Variables|/Game/IKTest/BP_MotionController.BP_MotionController_C|GetMotionController _output_get_2))))))
    (:then_2
      (Variables|Default|SetHandRTransform _returnvalue)
      (Variables|Default|SetHandLTransfrorm _returnvalue))))

(event Input|ActionEvents|InputActionGrabLeft
  (params (Key :type Key%20Structure))
  (bind _leftcontroller (Variables|Default|GetLeftController))
  (:Pressed
    (Default|GrabActor _leftcontroller))
  (:Released
    (Default|ReleaseActor _leftcontroller)))

(event Input|ActionEvents|InputActionGrabRight
  (params (Key :type Key%20Structure))
  (bind _rightcontroller (Variables|Default|GetRightController))
  (:Pressed
    (Default|GrabActor _rightcontroller))
  (:Released
    (Default|ReleaseActor _rightcontroller)))

(fn ConstructionScript)